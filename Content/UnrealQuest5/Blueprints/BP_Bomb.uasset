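; BP_Bomb is a bomb actor that explodes when it overlaps any actor other than its owner.
; Detonation clears the static mesh, plays an explosion sound and runs a timeline that scales the Explosion component before destroying the bomb.
; Living BP_CharacterBase actors that begin overlapping the scaling Explosion component take damage with a fixed weight, with no owner check.
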(event `self.ReceiveActorBeginOverlap`
  (params (OtherActor :type "Actor Object Reference"))
  (if (!= OtherActor (`self.OwnerActor`))
    (`self.Execute` OtherActor)))

(event `self.Execute`
  (params (TargetCharacter :type "Object Object Reference"))
  (`StaticMeshComponent.SetStaticMesh` (`self.StaticMesh`) null)
  (`GameplayStatics.PlaySoundAtLocation` "/Game/UnrealQuest5/Sound/Explosion.Explosion" (`self.K2_GetActorLocation`) (struct) 1.0 1.0 0.0 null null null null)
  (bind (_direction _explosion_scale) (`Timeline|タイムライン`)
    (:`Update`
      (`SceneComponent.SetRelativeScale3D` (`self.Explosion`) (* _explosion_scale (`KismetMathLibrary.Conv_DoubleToVector` 8.0))))
    (:`Finished`
      (`self.K2_DestroyActor`))))

(event `self.Explosion.OnComponentBeginOverlap`
  (params (OverlappedComponent :type "PrimitiveComponent Object Reference") (OtherActor :type "Actor Object Reference") (OtherComp :type "PrimitiveComponent Object Reference") (OtherBodyIndex :type Integer) (bFromSweep :type Boolean) (SweepResult :type "HitResult Structure (by ref)"))
  (bind _asbp_character_base (cast `/Game/UnrealQuest5/Blueprints/BP_CharacterBase` OtherActor))
  (if (not (`/Game/UnrealQuest5/Blueprints/BP_CharacterBase.isDead` _asbp_character_base))
    (`/Game/UnrealQuest5/Blueprints/BP_CharacterBase.Damage` _asbp_character_base (`self.Damage`) 100)))

(fn `UserConstructionScript`
  (`parent.UserConstructionScript`))