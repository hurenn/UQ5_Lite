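; Gameplay ability for the second attack in a tag-chained combo, apparently an older version judging by its name.
; On activation it waits for Attack.StartNextAttack, then clears Attack.EnableNextAttack and plays the AM_Attack02 montage.
; Montage notify ends re-add those loose tags by notify name to signal the next attack.
; Completion or interruption ends the ability, which clears Attack.StartNextAttack.
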(event `self.K2_ActivateAbility`
  (`AbilityTask_WaitGameplayTagAdded.WaitGameplayTagAdd` (struct :`TagName` "Attack.StartNextAttack") null ; SartNextAttackタグが付くまで待機
    (:`Added`
      (`AbilitySystemBlueprintLibrary.RemoveLooseGameplayTags` (`self.GetOwningActorFromActorInfo`) (`BlueprintGameplayTagLibrary.MakeLiteralGameplayTagContainer` (struct :`GameplayTags` (struct :`(TagName` "Attack.EnableNextAttack") :`(TagName` "Attack.StartNextAttack")))))
      (bind _notifyname (`|PlayMontage` (`self.GetOwningComponentFromActorInfo`) "/Game/UnrealQuest5/Characters/Mannequins/Animations/UQ5/AM_Attack02.AM_Attack02")
        (:`OnCompleted`
          (`self.K2_EndAbility` :!label _label))
        (:`OnInterrupted`
          (goto _label))
        (:`OnNotifyEnd`
          (switch `string` (`KismetStringLibrary.Conv_NameToString` _notifyname)
            (:`EnableNextAttack`
              (`AbilitySystemBlueprintLibrary.AddLooseGameplayTags` (`self.GetOwningActorFromActorInfo`) (`BlueprintGameplayTagLibrary.MakeGameplayTagContainerFromTag` (struct :`TagName` "Attack.EnableNextAttack"))))
            (:`StartNextAttack`
              (`AbilitySystemBlueprintLibrary.AddLooseGameplayTags` (`self.GetOwningActorFromActorInfo`) (`BlueprintGameplayTagLibrary.MakeGameplayTagContainerFromTag` (struct :`TagName` "Attack.StartNextAttack"))))))))))

(event `self.K2_OnEndAbility`
  (params (bWasCancelled :type Boolean))
  (`AbilitySystemBlueprintLibrary.RemoveLooseGameplayTags` (`self.GetOwningActorFromActorInfo`) (`BlueprintGameplayTagLibrary.MakeLiteralGameplayTagContainer` (struct :`GameplayTags` (struct :`(TagName` "Attack.StartNextAttack") :`(TagName` "Attack.EnableNextAttack"))))))