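; Base enemy character for UnrealQuest5, handling attacks, parries, damage reactions and death on top of its parent class.
; Hits landing during pre-attack with Guard above the hit's Weight become parries, playing effects and calling the player's slow-world; others pass to parent damage.
; Parry and damage reactions pause AI brain logic, then restart it.
; Death polls DeadEnable before running parent logic and setting a short lifespan.
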(event `Attack`
  ;[1 0 0 0.5] 攻撃
  (`|PlayMontage` (`self.Mesh`) "/Game/UnrealQuest5/Characters/Mannequins/Animations/UQ5/AM_Enemy_Attack01.AM_Enemy_Attack01" (`self.AttackSpeedRate`)))

(event `PlayParried`
  (bind _blade (`self.Blade`))
  (bind _braincomponent (`AIController.BrainComponent` (`AIBlueprintHelperLibrary.GetAIController` self)))
  (`NiagaraFunctionLibrary.SpawnSystemAtLocation` "/Game/UnrealQuest5/Effects/NS_ParryEffect1.NS_ParryEffect1" (+ (`SceneComponent.GetSocketLocation` _blade "None") (* (`SceneComponent.GetUpVector` _blade) (`KismetMathLibrary.Conv_DoubleToVector` 50.0))))
  (`BrainComponent.StopLogic` _braincomponent "")
  (`|PlayMontage` (`self.Mesh`) "/Game/UnrealQuest5/Characters/Mannequins/Animations/UQ5/AM_Enemy_Parried.AM_Enemy_Parried"
    (:`then`
      (`GameplayStatics.PlaySoundAtLocation` "/Game/UnrealQuest5/Sound/Parry.Parry" (0.0 0.0 0.0) (struct) 1.0 1.0 0.0 null null null null)
      (bind _asbp_uq5_player (cast `/Game/UnrealQuest5/Blueprints/BP_UQ5_Player` (`GameplayStatics.GetPlayerPawn` 0)))
      (`/Game/UnrealQuest5/Blueprints/BP_UQ5_Player.SetSlowWorld` _asbp_uq5_player self))
    (:`OnCompleted`
      (`BrainComponent.RestartLogic` _braincomponent))))

(event `self.PlayDamage`
  (bind _braincomponent (`AIController.BrainComponent` (`AIBlueprintHelperLibrary.GetAIController` self)))
  (`BrainComponent.StopLogic` _braincomponent "")
  (`parent.PlayDamage`)
  (`KismetSystemLibrary.Delay` 0.5)
  (`BrainComponent.RestartLogic` _braincomponent))

(event `self.PlayDead`
  (if (not (`self.DeadEnable`)) :!label _label
    (`KismetSystemLibrary.Delay` 0.1)
    (goto _label)
    (else
      (`parent.PlayDead`)
      (`self.SetLifeSpan` 1.5))))

(fn `Damage`
  (params (Damage :type Integer) (Weight :type Integer))
  (`self.SetAttackActive` false)
  (if (and (`self.IsPreAttack`) (> (`self.Guard`) Weight))
    (`self.PlayParried`)
    (else
      (`parent.Damage` Damage 100))))

(fn `SetMoveSpeed`
  (params (MoveSpeed :type "Float (double-precision)"))
  (set `CharacterMovementComponent.MaxWalkSpeed` MoveSpeed (`self.CharacterMovement`)))

(fn `UserConstructionScript`)