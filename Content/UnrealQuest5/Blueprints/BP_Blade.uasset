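; BP_Blade is a melee-style hit actor that damages characters it overlaps.
; On overlap it casts the other actor to BP_CharacterBase and skips any whose class is a child of its ParentClass value, filtering out that class family.
; Characters that are neither dead nor invincible receive a Damage call carrying the blade's AttackPower and AttackWeight.
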(event `self.ReceiveActorBeginOverlap`
  (params (OtherActor :type "Actor Object Reference"))
  (bind _asbp_character_base (cast `/Game/UnrealQuest5/Blueprints/BP_CharacterBase` OtherActor))
  (if (not (`KismetMathLibrary.ClassIsChildOf` (`GameplayStatics.GetObjectClass` OtherActor) (`self.ParentClass`)))
    (if (`/Game/UnrealQuest5/Blueprints/BP_CharacterBase.isDead` _asbp_character_base)
      _
      (elif (not (`/Game/UnrealQuest5/Blueprints/BP_CharacterBase.IsInvince` _asbp_character_base))
        (`/Game/UnrealQuest5/Blueprints/BP_CharacterBase.Damage` _asbp_character_base (`self.AttackPower`) (`self.AttackWeight`))))))

(fn `UserConstructionScript`
  (`parent.UserConstructionScript`))