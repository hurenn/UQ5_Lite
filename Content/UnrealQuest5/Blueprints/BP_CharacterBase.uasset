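; Base character Blueprint that handles HP, damage, recovery and death, and toggles collision on its Blade child-actor weapon.
; Damage spawns hit VFX and sound, lowers clamped HP and plays a damage montage, then triggers death at zero.
; Death disables movement, ragdolls the mesh and calls a dead event.
; Both reactions disable the attack and apply a brief global time-dilation hit-stop unless the player is in slow mode.
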(event `PlayDead`
  (set `self.isDead` true)
  (`self.SetAttackActive` false)
  (`CharacterMovementComponent.DisableMovement` (`self.CharacterMovement`))
  (`PrimitiveComponent.SetCollisionProfileName` (`self.Mesh`) "Ragdoll" true)
  (`PrimitiveComponent.SetSimulatePhysics` (`self.Mesh`) true)
  (`self.DeadEvent`)
  (bind _asbp_uq5_player (cast `/Game/UnrealQuest5/Blueprints/BP_UQ5_Player` (`GameplayStatics.GetPlayerPawn` 0)))
  (if (not (`/Game/UnrealQuest5/Blueprints/BP_UQ5_Player.IsSlow` _asbp_uq5_player))
    (`GameplayStatics.SetGlobalTimeDilation` (`KismetMathLibrary.FClamp` (* (`GameplayStatics.GetGlobalTimeDilation`) 0.05) 0.05))
    (`KismetSystemLibrary.DelayUntilNextTick`)
    (`KismetSystemLibrary.DelayUntilNextTick`)
    (`KismetSystemLibrary.Delay` 0.005)
    (`GameplayStatics.SetGlobalTimeDilation` (`KismetMathLibrary.FClamp` (/ (`GameplayStatics.GetGlobalTimeDilation`) 0.05) 0.05))))

(event `PlayDamage`
  (`self.SetAttackActive` false)
  (`|PlayMontage` (`self.Mesh`) "/Game/UnrealQuest5/Characters/Mannequins/Animations/UQ5/AM_Enemy_Damaged.AM_Enemy_Damaged"
    (:`then`
      (set `self.IsMontageMotion` true)
      (bind _asbp_uq5_player (cast `/Game/UnrealQuest5/Blueprints/BP_UQ5_Player` (`GameplayStatics.GetPlayerPawn` 0)))
      (if (not (`/Game/UnrealQuest5/Blueprints/BP_UQ5_Player.IsSlow` _asbp_uq5_player))
        (`GameplayStatics.SetGlobalTimeDilation` (`KismetMathLibrary.FClamp` (* (`GameplayStatics.GetGlobalTimeDilation`) 0.1) 0.05))
        (`KismetSystemLibrary.DelayUntilNextTick`)
        (`KismetSystemLibrary.DelayUntilNextTick`)
        (`KismetSystemLibrary.Delay` 0.005)
        (`GameplayStatics.SetGlobalTimeDilation` (`KismetMathLibrary.FClamp` (/ (`GameplayStatics.GetGlobalTimeDilation`) 0.1) 0.05))))
    (:`OnCompleted`
      (`self.SetMontageMortion` false))))

(event `self.ReceiveBeginPlay`
  (`parent.ReceiveBeginPlay`)
  (set `self.HP` (`self.MaxHP`)))

(fn `Damage`
  (params (Damage :type Integer) (Weight :type Integer :default 100))
  (`NiagaraFunctionLibrary.SpawnSystemAtLocation` "/Game/UnrealQuest5/Effects/NS_HitEffect.NS_HitEffect" (+ (`self.K2_GetActorLocation`) (0.0 20.0 0.0)))
  (`GameplayStatics.PlaySoundAtLocation` "/Game/UnrealQuest5/Sound/Damage.Damage" (0.0 0.0 0.0) (struct) 1.0 1.0 0.0 null null null null)
  (bind _output_get (set `self.HP` (`KismetMathLibrary.Clamp` (- (`self.HP`) Damage) 0 (`self.MaxHP`))))
  (`self.PlayDamage`)
  (if (not (> _output_get 0))
    (`self.PlayDead`)))

(fn `Recover`
  (params (Recover :type Integer))
  (set `self.HP` (`KismetMathLibrary.Clamp` (+ Recover (`self.HP`)) 0 (`self.MaxHP`))))

(fn `SetAttackActive`
  (params (Enable :type Boolean))
  (bind _asbp_weapon (cast `/Game/UnrealQuest5/Blueprints/BP_Weapon` (`ChildActorComponent.ChildActor` (`self.Blade`))))
  (`/Game/UnrealQuest5/Blueprints/BP_Weapon.SetCollisionActive` _asbp_weapon Enable))

(fn `SetMontageMortion`
  (params (SetMortion :type Boolean))
  (set `self.IsMontageMotion` SetMortion))

(fn `UserConstructionScript`)