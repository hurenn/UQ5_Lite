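; Base Gameplay Ability for chained attacks: plays a montage, flags the character as attacking and locks player movement until blend-out.
; Montage notify ends add loose EnableNextAttack and StartNextAttack tags to gate combos.
; Activation clears the former tag, ending clears the latter.
; IsWaitTag adds a StartNextAttack tag wait, but the montage is wired to its immediate exec pin, so playback does not wait.
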(event `self.K2_ActivateAbility`
  (`AbilitySystemBlueprintLibrary.RemoveLooseGameplayTags` (`self.GetOwningActorFromActorInfo`) (`BlueprintGameplayTagLibrary.MakeLiteralGameplayTagContainer` (struct :`GameplayTags` (struct :`(TagName` "Attack.EnableNextAttack")))))
  (if (`self.IsWaitTag`)
    (`AbilityTask_WaitGameplayTagAdded.WaitGameplayTagAdd` (struct :`TagName` "Attack.StartNextAttack") null ; SartNextAttackタグが付くまで待機
      (:`then`
        _)))
  (bind _notifyname (`|PlayMontage` (`self.GetOwningComponentFromActorInfo`) (`self.Montage Name`))
    (:`then`
      (bind _asbp_character_base (cast `/Game/UnrealQuest5/Blueprints/BP_CharacterBase` (`self.GetAvatarActorFromActorInfo`)))
      (set `/Game/UnrealQuest5/Blueprints/BP_CharacterBase.IsAttackMotion` true _asbp_character_base)
      (bind _asbp_uq5_player (cast `/Game/UnrealQuest5/Blueprints/BP_UQ5_Player` _asbp_character_base))
      (`/Game/UnrealQuest5/Blueprints/BP_UQ5_Player.SetCanMove` _asbp_uq5_player false))
    (:`OnCompleted`
      (set `/Game/UnrealQuest5/Blueprints/BP_CharacterBase.IsAttackMotion` false _asbp_character_base)
      (`self.K2_EndAbility`))
    (:`OnBlendOut`
      (bind _asbp_uq5_player_2 (cast `/Game/UnrealQuest5/Blueprints/BP_UQ5_Player` _asbp_character_base))
      (`/Game/UnrealQuest5/Blueprints/BP_UQ5_Player.SetCanMove` _asbp_uq5_player_2 true))
    (:`OnInterrupted`
      (`self.K2_EndAbility`))
    (:`OnNotifyEnd`
      (switch `string` (`KismetStringLibrary.Conv_NameToString` _notifyname)
        (:`EnableNextAttack`
          (`AbilitySystemBlueprintLibrary.AddLooseGameplayTags` (`self.GetOwningActorFromActorInfo`) (`BlueprintGameplayTagLibrary.MakeGameplayTagContainerFromTag` (struct :`TagName` "Attack.EnableNextAttack"))))
        (:`StartNextAttack`
          (`AbilitySystemBlueprintLibrary.AddLooseGameplayTags` (`self.GetOwningActorFromActorInfo`) (`BlueprintGameplayTagLibrary.MakeGameplayTagContainerFromTag` (struct :`TagName` "Attack.StartNextAttack"))))))))

(event `self.K2_OnEndAbility`
  (params (bWasCancelled :type Boolean))
  (`AbilitySystemBlueprintLibrary.RemoveLooseGameplayTags` (`self.GetOwningActorFromActorInfo`) (`BlueprintGameplayTagLibrary.MakeLiteralGameplayTagContainer` (struct :`GameplayTags` (struct :`(TagName` "Attack.StartNextAttack") :`(TagName` "Attack.EnableNextAttack"))))))