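; BP_Portion is a recovery item actor, apparently a potion, that restores the player character when used.
; Its Execute event casts the target character to BP_UQ5_Player, passes its Recover value to that player's Recover function, then destroys itself.
; A failed cast leaves the item in place, and the default BeginPlay, overlap, Tick and construction handlers add no logic of their own.
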(event `self.Execute`
  (params (TargetCharacter :type "Object Object Reference"))
  (bind _asbp_uq5_player (cast `/Game/UnrealQuest5/Blueprints/BP_UQ5_Player` TargetCharacter))
  (`/Game/UnrealQuest5/Blueprints/BP_CharacterBase.Recover` _asbp_uq5_player (`self.Recover`))
  (`self.K2_DestroyActor`))

(fn `UserConstructionScript`
  (`parent.UserConstructionScript`))