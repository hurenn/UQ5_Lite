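; Gameplay ability for the first attack of what appears to be a combo, playing the AM_Attack01 montage on the owner.
; Montage notifies add loose, non-replicated tags to the owning actor, marking when the next attack is enabled and when it should start.
; The ability ends when the montage completes or is interrupted.
; On end it removes only the Attack.StartNextAttack tag, leaving Attack.EnableNextAttack in place.
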(event `self.K2_ActivateAbility`
  (bind _notifyname (`|PlayMontage` (`self.GetOwningComponentFromActorInfo`) "/Game/UnrealQuest5/Characters/Mannequins/Animations/UQ5/AM_Attack01.AM_Attack01")
    (:`OnCompleted`
      (`self.K2_EndAbility` :!label _label))
    (:`OnInterrupted`
      (goto _label))
    (:`OnNotifyBegin`
      (switch `string` (`KismetStringLibrary.Conv_NameToString` _notifyname)
        (:`EnableNextAttack`
          (`AbilitySystemBlueprintLibrary.AddLooseGameplayTags` (`self.GetOwningActorFromActorInfo`) (`BlueprintGameplayTagLibrary.MakeGameplayTagContainerFromTag` (struct :`TagName` "Attack.EnableNextAttack"))))
        (:`StartNextAttack`
          (`AbilitySystemBlueprintLibrary.AddLooseGameplayTags` (`self.GetOwningActorFromActorInfo`) (`BlueprintGameplayTagLibrary.MakeGameplayTagContainerFromTag` (struct :`TagName` "Attack.StartNextAttack"))))))))

(event `self.K2_OnEndAbility`
  (params (bWasCancelled :type Boolean))
  (`AbilitySystemBlueprintLibrary.RemoveLooseGameplayTags` (`self.GetOwningActorFromActorInfo`) (`BlueprintGameplayTagLibrary.MakeLiteralGameplayTagContainer` (struct :`GameplayTags` (struct :`(TagName` "Attack.StartNextAttack") :`(TagName` "Attack.EnableNextAttack"))))))