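; Wave-style enemy spawner that also tracks the kill objective and announces a win once deaths reach MaxCount.
; On BeginPlay it creates the score widget, then uses the SpawnDelay macro to stagger five initial spawns.
; Spawn places random EnemyList picks inside the Box bounds, caps the lifetime total at MaxCount, and binds each death event.
; Each death updates the score, then either spawns again after SpawnTimer or prints "Win!" and plays the clear sound.
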(event `self.ReceiveBeginPlay`
  (`self.MakeWidgetScore`)
  (`self.SpawnDelay`)
  (`self.SpawnDelay`)
  (`self.SpawnDelay`)
  (`self.SpawnDelay`)
  (`self.SpawnDelay`))

(event `Spawn`
  (bind (_origin _boxextent) (`KismetSystemLibrary.GetComponentBounds` (`self.Box`)))
  (if (< (`self.CurrentCount`) (`self.MaxCount`))
    (set `self.CurrentCount` (+ (`self.CurrentCount`) 1))
    (bind _returnvalue (`|SpawnActorFromClass` (`KismetArrayLibrary.Array_Random` (`self.EnemyList`)) (`KismetMathLibrary.MakeTransform` (`KismetMathLibrary.RandomPointInBoundingBox` _origin _boxextent)) "Undefined" "OverrideRootScale" null null))
    (add `/Game/UnrealQuest5/Blueprints/BP_UQ5_Enemy_Base.DeadEvent` _returnvalue (delegate `EnemyDead`))))

(event `EnemyDead`
  (bind _output_get (set `self.DeathCount` (+ (`self.DeathCount`) 1)))
  (`TextBlock.SetText` (`/Game/ThirdPersonTemp/AI/WB_Score.CurrentCount` (`self.WB_Score`)) (`KismetTextLibrary.Conv_IntToText` _output_get))
  (if (>= (`self.DeathCount`) (`self.MaxCount`))
    (`KismetSystemLibrary.PrintString` "Win!")
    (`GameplayStatics.PlaySound2D` "/Game/UnrealQuest5/Sound/Clear.Clear" 1.0 1.0 0.0 null null)
    (else
      (`KismetSystemLibrary.Delay` (`self.SpawnTimer`))
      (`self.Spawn`))))

(fn `MakeWidgetScore`
  (bind _returnvalue (`|CreateWidget` "/Game/ThirdPersonTemp/AI/WB_Score.WB_Score_C"))
  (bind _output_get (set `self.WB_Score` _returnvalue))
  (`UserWidget.AddToViewport` _output_get 0)
  (`TextBlock.SetText` (`/Game/ThirdPersonTemp/AI/WB_Score.Total` (`self.WB_Score`)) (`KismetTextLibrary.Conv_IntToText` (`self.MaxCount`)))
  (`TextBlock.SetText` (`/Game/ThirdPersonTemp/AI/WB_Score.CurrentCount` (`self.WB_Score`)) "0"))

(fn `UserConstructionScript`)